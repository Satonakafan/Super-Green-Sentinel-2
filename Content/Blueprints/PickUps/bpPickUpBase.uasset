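; Base pickup Blueprint that drifts along the world Y axis until the player comes within range, then homes in on them.
; The first PickUpCollider overlap with a bpPlayer caches that player as the target, which is never cleared here.
; Each Tick sets the ProjectileMovement velocity, lerping it by a fixed alpha toward the player's direction at IncreaseSpeed for a smoothed, frame-rate-dependent turn.
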(event `self.ReceiveTick`
  (params (DeltaSeconds :type "Float (single-precision)"))
  (bind _projectilemovement (`self.ProjectileMovement`))
  ;[1 1 1] PickUp Movement - Controls the Movement of the PickUp Items
  ;;[1 1 1] Checks to see if the player has spawned/within range, at the time this will run it should return false
  (`/Engine/EditorBlueprintResources/StandardMacros.IsValid` (`self.bpPlayer`)
    (:`Is Valid`
      (set `MovementComponent.Velocity` (`KismetMathLibrary.VLerp` (`MovementComponent.Velocity` (`self.ProjectileMovement`)) (* (`KismetMathLibrary.Normal` (- (`self.K2_GetActorLocation` (`self.bpPlayer`)) (`self.K2_GetActorLocation`))) (`self.IncreaseSpeed`)) 0.1) _projectilemovement))
    (:`Is Not Valid`
      (set `MovementComponent.Velocity` (`KismetMathLibrary.MakeVector` 0.0 (`self.MovementSpeed`)) _projectilemovement))))

(event `self.PickUpCollider.OnComponentBeginOverlap`
  (params (OverlappedComponent :type "PrimitiveComponent Object Reference") (OtherActor :type "Actor Object Reference") (OtherComp :type "PrimitiveComponent Object Reference") (OtherBodyIndex :type Integer) (bFromSweep :type Boolean) (SweepResult :type "HitResult Structure (by ref)"))
  ;[1 1 1] Checks to see if a reference to the Player has already been made. When one is made then the PickUp Movement script will start
  (bind _asbp_player (cast `/Game/Blueprints/Essentials/bpPlayer` OtherActor))
  (`/Engine/EditorBlueprintResources/StandardMacros.IsValid` (`self.bpPlayer`)
    (:`Is Not Valid`
      (set `self.bpPlayer` _asbp_player))))

(fn `UserConstructionScript`)