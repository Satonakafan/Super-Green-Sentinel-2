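; Bomb pickup actor that adds one bomb to the player who touches it.
; When its PickUpMesh begins overlapping a bpPlayer, it increments BombNo if that is below MaxBombNo.
; The pickup then destroys itself, even if the player is already at the maximum.
; Tick and construction only call the parent class, and other overlapping actors are ignored.
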(event `self.ReceiveTick`
  (params (DeltaSeconds :type "Float (single-precision)"))
  (`parent.ReceiveTick` DeltaSeconds))

(event `self.PickUpMesh.OnComponentBeginOverlap`
  (params (OverlappedComponent :type "PrimitiveComponent Object Reference") (OtherActor :type "Actor Object Reference") (OtherComp :type "PrimitiveComponent Object Reference") (OtherBodyIndex :type Integer) (bFromSweep :type Boolean) (SweepResult :type "HitResult Structure (by ref)"))
  (bind _asbp_player (cast `/Game/Blueprints/Essentials/bpPlayer` OtherActor))
  (if (< (`/Game/Blueprints/Essentials/bpPlayer.BombNo` _asbp_player) (`/Game/Blueprints/Essentials/bpPlayer.MaxBombNo` _asbp_player))
    (`/Engine/EditorBlueprintResources/StandardMacros.IncrementInt` (`/Game/Blueprints/Essentials/bpPlayer.BombNo` _asbp_player)
      (:`  `
        _)))
  (`self.K2_DestroyActor`))

(fn `UserConstructionScript`
  (`parent.UserConstructionScript`))