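; Health pickup actor that restores one point of health or shield to the player on touch.
; When its pickup mesh begins overlapping a bpPlayer, it increments ShieldHealth if that player's shield is active, otherwise Health, then destroys itself.
; The increment has no cap check here, and Tick and the construction script only call their parent versions.
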(event `self.ReceiveTick`
  (params (DeltaSeconds :type "Float (single-precision)"))
  (`parent.ReceiveTick` DeltaSeconds))

(event `self.PickUpMesh.OnComponentBeginOverlap`
  (params (OverlappedComponent :type "PrimitiveComponent Object Reference") (OtherActor :type "Actor Object Reference") (OtherComp :type "PrimitiveComponent Object Reference") (OtherBodyIndex :type Integer) (bFromSweep :type Boolean) (SweepResult :type "HitResult Structure (by ref)"))
  ;[1 1 1] If this hits the player and their shield is not active then it will give them 1/3 health, if shield is active it will give them 1/3 shield health
  (bind _asbp_player (cast `/Game/Blueprints/Essentials/bpPlayer` OtherActor))
  (if (`/Game/Blueprints/Essentials/bpPlayer.bShieldActive` _asbp_player)
    (bind _result (`/Engine/EditorBlueprintResources/StandardMacros.IncrementFloat` (`/Game/Blueprints/Essentials/bpPlayer.ShieldHealth` _asbp_player))
      (:`  `
        (set `/Game/Blueprints/Essentials/bpPlayer.ShieldHealth` _result _asbp_player)))
    (else
      (bind _result_2 (`/Engine/EditorBlueprintResources/StandardMacros.IncrementFloat` (`/Game/Blueprints/Essentials/bpPlayer.Health` _asbp_player))
        (:`  `
          (set `/Game/Blueprints/Essentials/bpPlayer.Health` _result_2 _asbp_player)))))
  (`self.K2_DestroyActor`))

(fn `UserConstructionScript`
  (`parent.UserConstructionScript`))