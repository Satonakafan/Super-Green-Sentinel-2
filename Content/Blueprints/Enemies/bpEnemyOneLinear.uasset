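; Enemy ship Blueprint that repeatedly fires a single projectile in a straight line along negative Y.
; After the parent Tick, a Delay of FireRate acts as the fire timer, then a BpEnemyProjectileBase spawns at ProjectileSpawn with fixed damage, speed and scale.
; BeginPlay and construction only call the parent.
; Disconnected logic for hostile/passive mesh toggling and a player-death check never runs.
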(event `self.ReceiveBeginPlay`
  (`parent.ReceiveBeginPlay`))

(event `self.ReceiveTick`
  (params (DeltaSeconds :type "Float (single-precision)"))
  (`parent.ReceiveTick` DeltaSeconds)
  (`KismetSystemLibrary.Delay` (`self.FireRate`))
  (`|SpawnActorFromClass` "/Game/Blueprints/Projectiles/Enemy/bpEnemyProjectileBase.bpEnemyProjectileBase_C" (`SceneComponent.K2_GetComponentToWorld` (`self.ProjectileSpawn`)) "AdjustIfPossibleButAlwaysSpawn" "OverrideRootScale" null 1.0 (0.0 -2000.0 0.0) (10.0 12.5 10.0) null))

(fn `UserConstructionScript`
  (`parent.UserConstructionScript`))