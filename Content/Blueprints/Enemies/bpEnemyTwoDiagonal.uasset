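; Enemy Blueprint that repeatedly fires a pair of projectiles from its Top and Bottom components.
; Tick runs the parent logic, then uses a Delay of FireRate as a repeating fire timer.
; Each cycle spawns two BpEnemyProjectileBase actors at those component transforms, with identical damage, scale and negative-Y speed vector.
; BeginPlay and overlap events are disabled stubs, and construction only calls the parent.
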(event `self.ReceiveTick`
  (params (DeltaSeconds :type "Float (single-precision)"))
  (`parent.ReceiveTick` DeltaSeconds)
  (`KismetSystemLibrary.Delay` (`self.FireRate`))
  (`|SpawnActorFromClass` "/Game/Blueprints/Projectiles/Enemy/bpEnemyProjectileBase.bpEnemyProjectileBase_C" (`SceneComponent.K2_GetComponentToWorld` (`self.Top`)) "AdjustIfPossibleButAlwaysSpawn" "OverrideRootScale" null 1.0 (0.0 -2000.0 0.0) (15.0 15.0 15.0) null)
  (`|SpawnActorFromClass` "/Game/Blueprints/Projectiles/Enemy/bpEnemyProjectileBase.bpEnemyProjectileBase_C" (`SceneComponent.K2_GetComponentToWorld` (`self.Bottom`)) "AdjustIfPossibleButAlwaysSpawn" "OverrideRootScale" null 1.0 (0.0 -2000.0 0.0) (15.0 15.0 15.0) null))

(fn `UserConstructionScript`
  (`parent.UserConstructionScript`))