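; Enemy wave spawner that runs a sequence of ten waves, each with its own enemy count and class pool.
; A looping timer calls WaveChecker, which starts the next wave when the game mode reports no active enemies and WaveReady is set, with a delay before the last.
; StartWave publishes the count to the game mode.
; SpawnWave spawns random pool picks at fixed X/Y and random Z within game mode bounds.
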(event `self.ReceiveBeginPlay`
  ;[1 1 1] Sets the timer that controls the enemy waves spawning
  (bind _asbp_game_mode (cast `/Game/Blueprints/Essentials/bpGameMode` (`GameplayStatics.GetGameMode`)))
  (set `self.bpGameMode` _asbp_game_mode)
  ;;[1 1 1] Timers are similar to an EventTick which can be run repeatedly by ticking the looping option. In this instance it has been set to repeat every 0.5 seconds
  (bind _returnvalue (`KismetSystemLibrary.K2_SetTimer` null "WaveChecker" 0.5 true))
  (set `self.WaveTimer` _returnvalue))

(event `WaveChecker`
  (bind _output (`|GetArrayItem` (`self.EnemyWaveCount`) (`self.WaveIndex`)))
  ;[1 1 1] Wave Checker - Controls the enemies spawning
  (if (and (== (`/Game/Blueprints/Essentials/bpGameMode.ActiveEnemies` (`self.bpGameMode`)) 0) (`self.bWaveReady`))
    (switch `int` (`self.WaveIndex`)
      (:`0`
        (`self.StartWave` _output)
        ;;[1 1 1 1 15] Wave Total: Controls amount of enemies spawned in wave 1
        ;; Enemy Wave: Controls type of enemies in wave 1
        (`self.SpawnWave` _output (`self.EnemyWave1`)))
      (:`1`
        (`self.StartWave` _output)
        (`self.SpawnWave` _output (`self.EnemyWave2`)))
      (:`2`
        (`self.StartWave` _output)
        (`self.SpawnWave` _output (`self.EnemyWave3`)))
      (:`3`
        (`self.StartWave` _output)
        (`self.SpawnWave` _output (`self.EnemyWave4`)))
      (:`4`
        (`self.StartWave` _output)
        (`self.SpawnWave` _output (`self.EnemyWave5`)))
      (:`5`
        (`self.StartWave` _output)
        (`self.SpawnWave` _output (`self.EnemyWave6`)))
      (:`6`
        (`self.StartWave` _output)
        (`self.SpawnWave` _output (`self.EnemyWave7`)))
      (:`7`
        (`self.StartWave` _output)
        (`self.SpawnWave` _output (`self.EnemyWave8`)))
      (:`8`
        (`self.StartWave` _output)
        (`self.SpawnWave` _output (`self.EnemyWave9`)))
      (:`9`
        (`KismetSystemLibrary.Delay` 2.0)
        (`self.StartWave` _output)
        (`self.SpawnWave` _output (`self.EnemyWave10`))))
    ;;[1 1 1] Keeps track of which wave is currently active
    (set `self.WaveIndex` (+ (`self.WaveIndex`) 1))))

(fn `SpawnWave`
  (params (WaveTotal :type Integer) (EnemyWave :type "Array of /Game/Blueprints/Enemies/bpEnemyBase Class Reference"))
  (bind _bpgamemode (`self.bpGameMode`))
  (bind (_enemyspawnlocationmin_x _enemyspawnlocationmin_y _enemyspawnlocationmin_z) (`KismetMathLibrary.BreakVector` (`/Game/Blueprints/Essentials/bpGameMode.EnemySpawnLocationMin` _bpgamemode)))
  (bind (_enemyspawnlocationmax_x _enemyspawnlocationmax_y _enemyspawnlocationmax_z) (`KismetMathLibrary.BreakVector` (`/Game/Blueprints/Essentials/bpGameMode.EnemySpawnLocationMax` _bpgamemode)))
  ;[1 1 1] On every loop this will check to see if there are currently more enemies alive than in the current wave
  (for _ (range (+ (+ WaveTotal 1) 1))
    (if (> WaveTotal (`self.ActiveWave`))
      (if (not (`self.bWaveReady`))
        (`|SpawnActorFromClass` (`|GetArrayItem` EnemyWave (`KismetMathLibrary.RandomInteger` (`KismetArrayLibrary.Array_Length` EnemyWave))) (`KismetMathLibrary.MakeTransform` (`KismetMathLibrary.MakeVector` _enemyspawnlocationmin_x _enemyspawnlocationmin_y (`KismetMathLibrary.RandomFloatInRange` _enemyspawnlocationmin_z _enemyspawnlocationmax_z))) "Undefined" "OverrideRootScale" null null)
        (set `self.ActiveWave` (+ (`self.ActiveWave`) 1)))
      (else
        (set `self.bWaveReady` true)))))

(fn `StartWave`
  (params (WaveTotal :type Integer))
  (bind _bpgamemode (`self.bpGameMode`))
  (set `self.bWaveReady` false)
  (set `self.ActiveWave` 0)
  (set `/Game/Blueprints/Essentials/bpGameMode.MaxWaves` WaveTotal _bpgamemode)
  (set `/Game/Blueprints/Essentials/bpGameMode.ActiveWave` WaveTotal _bpgamemode))

(fn `UserConstructionScript`)