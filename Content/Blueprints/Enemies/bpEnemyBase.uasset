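; Base enemy Blueprint that bounces around the level, damages the player on contact and reports itself to bpGameMode's ActiveEnemies count.
; A timeline sweeps it in along Y, then Tick moves it diagonally in Y/Z at random speed.
; Non-enemy hits flip Z and randomise Y direction.
; Ramming the player or losing all health shares one death path: decrement count, drop score item and chance-based random pickup, explode, destroy.
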(event `self.ReceiveBeginPlay`
  (bind _spawnlocation (`self.SpawnLocation`))
  ;[1 1 1] Movement Direction (Via Random Controls)
  (bind _asbp_game_mode (cast `/Game/Blueprints/Essentials/bpGameMode` (`GameplayStatics.GetGameMode`)))
  ;;[1 1 1] Tells the GameMode that another enemy has been called by updating the ActiveEnemies Variable
  (bind _output_get (set `self.bpGameMode` _asbp_game_mode))
  (set `/Game/Blueprints/Essentials/bpGameMode.ActiveEnemies` (+ (`/Game/Blueprints/Essentials/bpGameMode.ActiveEnemies` _output_get) 1) _output_get)
  ;;[1 1 1] Returns the value so that it can be used when deciding the enemies movement pattern
  (set `self.bMovementDirection` (`KismetMathLibrary.RandomBool`))
  ;;[1 1 1] Randomises the Enemies movement whilst moving. Adds variety
  (set `self.MovementSpeed` (`KismetMathLibrary.RandomFloatInRange` 500.0 1000.0))
  (set `self.SweepIn` (`KismetMathLibrary.RandomFloatInRange` 1200.0 1700.0))
  ;[1 1 1] Spawn Animation
  (set `self.SpawnLocation` (`self.K2_GetActorLocation`))
  (bind (_direction _speed) (`Timeline|EnemySpawnAnimation`)
    (:`Update`
      (`self.K2_SetActorLocation` (`KismetMathLibrary.VLerp` _spawnlocation (- _spawnlocation (`KismetMathLibrary.MakeVector` 0.0 (`self.SweepIn`))) _speed)))
    (:`Finished`
      (set `self.bMovementEnabled` true))))

(event `self.ReceiveTick`
  (params (DeltaSeconds :type "Float (single-precision)"))
  (if (`self.bMovementEnabled`)
    (`self.K2_SetActorLocation` (+ (`self.K2_GetActorLocation`) (* (`KismetMathLibrary.GreaterGreater_VectorRotator` (`KismetMathLibrary.MakeVector` 0.0 (* (`self.MovementSpeed`) (`KismetMathLibrary.SelectFloat` 1.0 -1.0 (`self.bMovementDirection_Y`))) (* (`self.MovementSpeed`) (`KismetMathLibrary.SelectFloat` 1.0 -1.0 (`self.bMovementDirection`))))) DeltaSeconds)) true)))

(event `self.ReceiveHit`
  (params (MyComp :type "PrimitiveComponent Object Reference") (Other :type "Actor Object Reference") (OtherComp :type "PrimitiveComponent Object Reference") (bSelfMoved :type Boolean) (HitLocation :type "Vector Structure") (HitNormal :type "Vector Structure") (NormalImpulse :type "Vector Structure") (Hit :type "HitResult Structure (by ref)"))
  (bind _bpgamemode (`self.bpGameMode`))
  (bind _pickuparray (`self.PickUpArray`))
  ;[1 1 1 1 17] Checks if the object this hit is of type enemy blueprint. If it's not then it will set the bool MovementDirection to the opposite of what it currently is. This is how the movement for the enemy will change when it hits a wall.
  (cast `/Game/Blueprints/Enemies/bpEnemyBase` Other
    (:`CastFailed`
      (set `self.bMovementDirection` (not (`self.bMovementDirection`)))
      ;[1 0 0.1519] add check to see if high difficulty or stage > 1
      (set `self.bMovementDirection_Y` (`KismetMathLibrary.RandomBool`))
      ;[1 1 1] If it hits the Player then it will do 1 point of damage
      (bind _asbp_player (cast `/Game/Blueprints/Essentials/bpPlayer` Other))
      (`GameplayStatics.ApplyDamage` _asbp_player 1.0)
      ;[1 1 1] Health Damage and Death
      ;;[1 1 1] If the enemies health is less than or equal to 0 then it is considered dead and this blueprint will cast to the game mode and minus 1 from the current amount of enemies alive before it destroys itself
      (set `/Game/Blueprints/Essentials/bpGameMode.ActiveEnemies` (- (`/Game/Blueprints/Essentials/bpGameMode.ActiveEnemies` _bpgamemode) 1) _bpgamemode :!label _label)
      (`|SpawnActorFromClass` "/Game/Blueprints/PickUps/bpPickUpScoreItem.bpPickUpScoreItem_C" (`self.GetTransform`) "Undefined" "OverrideRootScale" null null)
      (if (<= (`KismetMathLibrary.RandomFloatInRange` 0.0 1.0) (`self.DropRate`))
        (`|SpawnActorFromClass` (`|GetArrayItem` _pickuparray (`KismetMathLibrary.RandomIntegerInRange` 0 (`KismetArrayLibrary.Array_LastIndex` _pickuparray))) (`self.GetTransform`) "Undefined" "OverrideRootScale" null null))
      (`GameplayStatics.SpawnEmitterAtLocation` "/Game/Particles/pDeathExplosionEnemy.pDeathExplosionEnemy" (`self.K2_GetActorLocation`))
      (`KismetSystemLibrary.Delay` 0.1)
      (`self.K2_DestroyActor`))))

(event `self.ReceiveAnyDamage`
  (params (Damage :type "Float (single-precision)") (DamageType :type "DamageType Object Reference") (InstigatedBy :type "Controller Object Reference") (DamageCauser :type "Actor Object Reference"))
  ;[1 1 1] Health Damage and Death
  (set `self.Health` (`KismetMathLibrary.FClamp` (- (`self.Health`) Damage) 0.0 (`self.MaxHealth`)))
  ;;[1 1 1] If the enemies health is less than or equal to 0 then it is considered dead and this blueprint will cast to the game mode and minus 1 from the current amount of enemies alive before it destroys itself
  (if (<= (`self.Health`) 0.0)
    (goto _label)))

(fn `UserConstructionScript`
  (set `self.Health` (`self.MaxHealth`)))