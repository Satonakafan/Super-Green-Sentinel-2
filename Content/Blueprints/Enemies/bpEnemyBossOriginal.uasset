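; Two-phase boss enemy that fires projectiles and flags its defeat on the game mode.
; Tick uses a Delay as the fire-rate timer, spawning one shot from FirePoint, then at half health swapping meshes and firing faster from Top and Bottom.
; At zero health it destroys active enemy projectiles, setting IsBossDead inside that loop.
; The boss health widget and explosion emitter nodes are never run.
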(event `self.ReceiveBeginPlay`
  (`parent.ReceiveBeginPlay`))

(event `self.ReceiveTick`
  (params (DeltaSeconds :type "Float (single-precision)"))
  (`parent.ReceiveTick` DeltaSeconds)
  (if (<= (`self.Health`) 0.0)
    (bind _outactors (`GameplayStatics.GetAllActorsOfClass` "/Game/Blueprints/Projectiles/Enemy/bpEnemyProjectileBase.bpEnemyProjectileBase_C"))
    (for _array_element _outactors
      (`self.K2_DestroyActor` _array_element)
      (bind _asbp_game_mode (cast `/Game/Blueprints/Essentials/bpGameMode` (`GameplayStatics.GetGameMode`)))
      (set `/Game/Blueprints/Essentials/bpGameMode.bIsBossDead` true _asbp_game_mode))
    (else
      (`KismetSystemLibrary.Delay` (`self.FireRate`))
      (if (<= (`self.Health`) (/ (`self.MaxHealth`) 2.0))
        ;[1 1 1] Phase 2 attacks
        (`SceneComponent.SetVisibility` (`self.Phase1Mesh`) false false)
        (`SceneComponent.SetVisibility` (`self.EnemyMesh`) true false)
        (set `self.FireRate` 0.25)
        (`|SpawnActorFromClass` "/Game/Blueprints/Projectiles/Enemy/bpEnemyProjectileBase.bpEnemyProjectileBase_C" (`SceneComponent.K2_GetComponentToWorld` (`self.Top`)) "AdjustIfPossibleButAlwaysSpawn" "OverrideRootScale" null 0.5 (0.0 -2000.0 0.0) (15.0 15.0 15.0) null)
        (`|SpawnActorFromClass` "/Game/Blueprints/Projectiles/Enemy/bpEnemyProjectileBase.bpEnemyProjectileBase_C" (`SceneComponent.K2_GetComponentToWorld` (`self.Bottom`)) "AdjustIfPossibleButAlwaysSpawn" "OverrideRootScale" null 0.5 (0.0 -2000.0 0.0) (15.0 15.0 15.0) null)
        (else
          ;[1 1 1] Phase 1 attacks
          (`|SpawnActorFromClass` "/Game/Blueprints/Projectiles/Enemy/bpEnemyProjectileBase.bpEnemyProjectileBase_C" (`SceneComponent.K2_GetComponentToWorld` (`self.FirePoint`)) "AdjustIfPossibleButAlwaysSpawn" "OverrideRootScale" null 0.5 (0.0 -2000.0 0.0) (15.0 15.0 15.0) null))))))

(fn `UserConstructionScript`
  (`parent.UserConstructionScript`))