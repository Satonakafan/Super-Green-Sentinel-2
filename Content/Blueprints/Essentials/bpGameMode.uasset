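; Game mode that keeps the score and shows the win screen after the boss dies.
; Tick polls IsBossDead, waits three seconds, then adds a YouWin widget, shows the mouse cursor and sets game-and-UI input.
; The flag is never cleared here, so the widget is created again after each delay while it stays true.
; AddScore raises Score by a fixed amount per call.
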(event `self.ReceiveTick`
  (params (DeltaSeconds :type "Float (single-precision)"))
  (bind _returnvalue (`GameplayStatics.GetPlayerController` 0))
  (if (`self.bIsBossDead`)
    (`KismetSystemLibrary.Delay` 3.0)
    (bind _returnvalue_2 (`|CreateWidget` "/Game/Blueprints/UI/YouWin.YouWin_C"))
    (bind _output_get (set `self.YouWinRef` _returnvalue_2))
    (`UserWidget.AddToViewport` _output_get 0)
    (set `PlayerController.bShowMouseCursor` true _returnvalue)
    (`WidgetBlueprintLibrary.SetInputMode_GameAndUIEx` _returnvalue (`self.YouWinRef`))))

(fn `AddScore`
  (set `self.Score` (+ (`self.Score`) 10)))

(fn `UserConstructionScript`)