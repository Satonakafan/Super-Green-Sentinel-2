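; Player ship Blueprint for a shooter: flies in with a spinning timeline intro, then handles movement, firing, shield, bomb, pause and HUD.
; Tick eases horizontal and vertical speed with FInterpTo, moves with sweep and tilts the mesh.
; A cooldown and input-driven Gate handle held fire, single or toggleable double shot.
; Bombs clear enemy projectiles; damage drains an active shield, otherwise health, ending in Game Over and destruction.
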(event `self.ReceiveBeginPlay`
  (bind _spawnlocation (`self.SpawnLocation`))
  ;[1 1 1] Spawn Animation
  (`SceneComponent.SetVisibility` (`self.ShieldMesh`) false false)
  (bind _returnvalue (`GameplayStatics.GetCurrentLevelName` true))
  (if (`KismetStringLibrary.NotEqual_StrStr` _returnvalue "MainMenu")
    (set `self.Health` (`self.MaxHealth`))
    (set `self.BombNo` 1)
    (bind _returnvalue_2 (`|CreateWidget` "/Game/Blueprints/UI/HUD.HUD_C"))
    (bind _output_get (set `self.HUDRef` _returnvalue_2))
    (`UserWidget.AddToViewport` _output_get 0))
  (set `self.Pitch` (.pitch (`SceneComponent.RelativeRotation` (`self.PlayerMesh`))))
  ;;[1 1 1] Gets the rotation value of the PlayerMesh
  (set `self.SpawnRoation` (`SceneComponent.K2_GetComponentRotation` (`self.PlayerMesh`)))
  ;;[1 1 1] Sets the location to be the same as the value stored in the PlayerStart function
  (set `self.SpawnLocation` (`self.K2_GetActorLocation`))
  (bind (_direction _spawn) (`Timeline|PlayerSpawnAnimation`)
    (:`Update`
      (`self.K2_SetActorLocation` (`KismetMathLibrary.VLerp` _spawnlocation (+ _spawnlocation (0.0 2000.0 0.0)) _spawn))
      ;;[1 1 1] This tells the engine to only move the player mesh as opposed to the entire blueprint
      (`SceneComponent.K2_SetRelativeRotation` (`self.PlayerMesh`) (`KismetMathLibrary.RLerp` (`self.SpawnRoation`) (`KismetMathLibrary.MakeRotator` 0.0 (+ (`self.AnimationPitch`) (`self.Pitch`))) _spawn) false false))
    (:`Finished`
      (set `self.bCanMove` true)
      (set `self.bCanUseBomb` true))))

(event `self.ReceiveTick`
  (params (DeltaSeconds :type "Float (single-precision)"))
  ;[1 1 1] PlayerMovement
  (set `self.DeltaSeconds` DeltaSeconds)
  (if (`self.bCanMove`)
    (`self.FireRateController`)
    (`|ExecutionSequence`
      (:`then_0`
        (bind _returndirection (`self.GetDirection` (`self.SpeedVertical`) (`self.GetInputAxisValue`)))
        (set `self.SpeedVertical` _returndirection))
      (:`then_1`
        (bind _returndirection_2 (`self.GetDirection` (`self.SpeedHorizontal`) (`self.GetInputAxisValue`)))
        (set `self.SpeedHorizontal` _returndirection_2))
      (:`then_2`
        ;;[1 1 1] Controls the ships movement when the Move Up axis Mapping buttons are pressed.
        ;; In this instance if W is pressed then the ship moves up and if S is pressed then it
        ;; will move down.
        (`self.K2_SetActorLocation` (+ (`self.K2_GetActorLocation`) (`KismetMathLibrary.MakeVector` 0.0 0.0 (`self.SpeedVertical`))) true)
        ;;[1 1 1] Controls the ships movement when the Move Right axis Mapping buttons are pressed. In this instance if A is pressed then the ship moves left and if D is pressed then it will move right.
        (`self.K2_SetActorLocation` (+ (`self.K2_GetActorLocation`) (`KismetMathLibrary.MakeVector` 0.0 (`self.SpeedHorizontal`))) true)
        ;;[1 1 1] Adds a pitch to the player mesh when it is moving up or down. this is just a visual thing that looks nice
        (if (> (`self.Health`) 0.0)
          (`SceneComponent.K2_SetRelativeRotation` (`self.PlayerMesh`) (`KismetMathLibrary.RInterpTo` (`self.K2_GetActorRotation`) (`KismetMathLibrary.MakeRotator` 0.0 (`self.SpeedVertical`)) (`self.DeltaSeconds`) 80.0) false false))))))

(event `InputAction|SwapWeapon`
  (params (Key :type "Key Structure"))
  ;[1 1 1] Player Controller
  ;;[1 1 1] Player Shots - Controls the players firing
  (:`Pressed`
    (if (`self.bCanUseDoubleShot`)
      (`/Engine/EditorBlueprintResources/StandardMacros.FlipFlop`
        (:`A`
          (set `self.bDoubleShotActive` true))
        (:`B`
          (set `self.bDoubleShotActive` false))))))

(event `FireRateController`
  ;[1 1 1] Player Controller
  ;;[1 1 1] Player Shots - Controls the players firing
  (`|ExecutionSequence`
    (:`then_0`
      (set `self.PrimaryFireRate` (- (`self.PrimaryFireRate`) (`self.DeltaSeconds`)))
      (if (<= (`self.PrimaryFireRate`) 0.0)
        (`/Engine/EditorBlueprintResources/StandardMacros.Gate` true :!label _label
          (:`Exit`
            (set `self.PrimaryFireRate` (`self.PrimaryFireRateBase`))
            (if (`self.bDoubleShotActive`)
              (`self.PrimaryFire` (`self.ProjectileSpawnDoubleTop`))
              (`self.PrimaryFire` (`self.ProjectileSpawnDoubleBottom`))
              (else
                (`self.PrimaryFire` (`self.ProjectileSpawn`))))))))))

(event `InputAction|PrimaryFire`
  (params (Key :type "Key Structure"))
  ;[1 1 1] Player Controller
  ;;[1 1 1] Player Shots - Controls the players firing
  (:`Pressed`
    (goto _label :!via `Open`))
  (:`Released`
    (goto _label :!via `Close`)))

(event `InputAction|Shield`
  (params (Key :type "Key Structure"))
  ;[1 1 1] Player Controller
  ;;[1 1 1] Shield - Protects the Player from enemy bullets
  (:`Pressed`
    (if (`self.bCanUseShield`)
      (set `self.bCanUseShield` false)
      (`SceneComponent.ToggleVisibility` (`self.ShieldMesh`) false)
      (set `self.bShieldActive` true)
      (set `self.ShieldHealth` (`self.MaxShieldHealth`)))))

(event `InputAction|Bomb`
  (params (Key :type "Key Structure"))
  ;[1 1 1] Player Controller
  ;;[1 1 1] Bomb - Destroys all enemy bullets
  (:`Pressed`
    (if (and (> (`self.BombNo`) 0) (`self.bCanUseBomb`))
      (`/Engine/EditorBlueprintResources/StandardMacros.DecrementInt` (`self.BombNo`)
        (:`  `
          (bind _outactors (`GameplayStatics.GetAllActorsOfClass` "/Game/Blueprints/Projectiles/Enemy/bpEnemyProjectileBase.bpEnemyProjectileBase_C"))
          (for _array_element _outactors
            (`self.K2_DestroyActor` _array_element)
            (`GameplayStatics.SpawnEmitterAtLocation` "/Game/Particles/pExplosionBomb.pExplosionBomb" (4500.0 0.0 0.0))
            (set `self.bCanUseBomb` false)
            (`KismetSystemLibrary.Delay` 2.0)
            (set `self.bCanUseBomb` true)))))))

(event `InputAction|Pause`
  (params (Key :type "Key Structure"))
  (bind _returnvalue (`GameplayStatics.GetPlayerController` 0))
  ;[1 1 1] Player Controller
  ;;[1 1 1] Pause - Pauses the game
  (:`Pressed`
    (bind _returnvalue_2 (`|CreateWidget` "/Game/Blueprints/UI/PauseMenu.PauseMenu_C"))
    (bind _output_get (set `self.PauseMenuRef` _returnvalue_2))
    (`UserWidget.AddToViewport` _output_get 0)
    (set `PlayerController.bShowMouseCursor` true _returnvalue)
    (`WidgetBlueprintLibrary.SetInputMode_UIOnlyEx` _returnvalue (`self.PauseMenuRef`))
    (`GameplayStatics.SetGamePaused` true)))

(event `self.ReceiveAnyDamage`
  (params (Damage :type "Float (single-precision)") (DamageType :type "DamageType Object Reference") (InstigatedBy :type "Controller Object Reference") (DamageCauser :type "Actor Object Reference"))
  (bind _returnvalue (`GameplayStatics.GetPlayerController` 0))
  ;[0.9783 0.9366 1] Player Health
  (if (`self.bShieldActive`)
    (set `self.ShieldHealth` (`KismetMathLibrary.FClamp` (- (`self.ShieldHealth`) Damage) 0.0 (`self.MaxShieldHealth`)))
    (if (<= (`self.ShieldHealth`) 0.0)
      (`GameplayStatics.SpawnEmitterAtLocation` "/Game/Particles/pDeathExplosionPlayer.pDeathExplosionPlayer" (`self.K2_GetActorLocation`))
      (`SceneComponent.ToggleVisibility` (`self.ShieldMesh`) false)
      (set `self.bShieldActive` false)
      (set `self.bCanUseShield` false))
    (else
      (set `self.Health` (`KismetMathLibrary.FClamp` (- (`self.Health`) Damage) 0.0 (`self.MaxHealth`)))
      (if (<= (`self.Health`) 0.0)
        (bind _asbp_game_mode (cast `/Game/Blueprints/Essentials/bpGameMode` (`GameplayStatics.GetGameMode`)))
        (set `/Game/Blueprints/Essentials/bpGameMode.bIsPlayerDead` true _asbp_game_mode)
        (bind _returnvalue_2 (`|CreateWidget` "/Game/Blueprints/UI/GameOver.GameOver_C"))
        (bind _output_get (set `self.GameOverMenuRef` _returnvalue_2))
        (`UserWidget.AddToViewport` _output_get 0)
        (set `PlayerController.bShowMouseCursor` true _returnvalue)
        (`WidgetBlueprintLibrary.SetInputMode_GameAndUIEx` _returnvalue (`self.GameOverMenuRef`))
        (`GameplayStatics.SpawnEmitterAtLocation` "/Game/Particles/pDeathExplosionPlayer.pDeathExplosionPlayer" (`self.K2_GetActorLocation`))
        (`self.K2_DestroyActor`)))))

(event `InputAction|AddShield`
  (params (Key :type "Key Structure"))
  ;[1 1 1] Testing:
  ;;[1 1 1] Adds and Decreases shield
  (:`Pressed`
    (`/Engine/EditorBlueprintResources/StandardMacros.FlipFlop`
      (:`A`
        (if true
          (set `self.bCanUseShield` true)))
      (:`B`
        (if true
          (set `self.bCanUseShield` false))))))

(fn `GetDirection`
  (params (Speed :type "Float (double-precision)") (Direction :type "Float (double-precision)"))
  (returns (ReturnDirection :type "Float (double-precision)"))
  (bind _deltaseconds (`self.DeltaSeconds`))
  (bind _output_get (set `self.CurrentSpeed` (`KismetMathLibrary.FInterpTo` Speed (* (* Direction (`self.MovementSpeed`)) _deltaseconds) _deltaseconds 4.0)))
  (return _output_get))

(fn `PrimaryFire`
  (params (SpawnLocation :type "SceneComponent Object Reference"))
  (`|SpawnActorFromClass` "/Game/Blueprints/Projectiles/Player/bpPlayerProjectilePrimary.bpPlayerProjectilePrimary_C" (`KismetMathLibrary.MakeTransform` (.location (`SceneComponent.K2_GetComponentToWorld` SpawnLocation)) (.rotation (`SceneComponent.K2_GetComponentToWorld` SpawnLocation))) "AlwaysSpawn" "OverrideRootScale" null null))

(fn `ShieldActivate`
  (params (SpawnLocation :type "SceneComponent Object Reference"))
  (`|SpawnActorFromClass` "/Game/Blueprints/Essentials/bpPlayerShield.bpPlayerShield_C" (`KismetMathLibrary.MakeTransform` (.location (`SceneComponent.K2_GetComponentToWorld` SpawnLocation)) (.rotation (`SceneComponent.K2_GetComponentToWorld` SpawnLocation))) "AlwaysSpawn" "OverrideRootScale" null null))

(fn `UserConstructionScript`)